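; BP_Sphere is a keyboard-rotated sphere that ends the level by sending its child actor to a door.
; W/A/S/D rotate the root through Delay loops while held.
; The first press also calls PlayDetection on the BP_Platform actors gathered in the Construction Script, passing itself and their count.
; PlayAnimation disables input, eases ChildActor toward Door, then opens Level2 from Level1 or otherwise quits.
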(event `self.ReceiveBeginPlay`
  (`self.EnableInput` (`GameplayStatics.GetPlayerController` 0)))

(event `Key|A`
  (params (Key :type "Key Structure"))
  (:`Pressed`
    (if (`self.PlayerMoved`)
      ;[0 0.1472 0.15 0.5] Rotate Left
      (set `self.RotatingLeft` true :!label _label)
      (if (`self.RotatingLeft`) :!label _label_2
        (set `self.Rotation` (struct :`Yaw` 1.0))
        (`SceneComponent.K2_AddWorldRotation` (`self.DefaultSceneRoot`) (`self.Rotation`) false false)
        (`KismetSystemLibrary.Delay` 0.01)
        (goto _label_2))
      (else
        (set `self.PlayerMoved` true)
        (for _array_element (`self.Platforms`)
          (`/Engine/EditorBlueprintResources/StandardMacros.IsValid` _array_element
            (:`Is Valid`
              (`/Game/Blueprints/BP_Platform.PlayDetection` _array_element self (`KismetArrayLibrary.Array_Length` (`self.Platforms`)))
              (goto _label)))))))
  (:`Released`
    (set `self.RotatingLeft` false)))

(event `Key|D`
  (params (Key :type "Key Structure"))
  (:`Pressed`
    (if (`self.PlayerMoved`)
      ;[0.15 0 0 0.5] Rotate Right
      (set `self.RotatingRight` true :!label _label_3)
      (if (`self.RotatingRight`) :!label _label_4
        (set `self.Rotation` (struct :`Yaw` -1.0))
        (`SceneComponent.K2_AddWorldRotation` (`self.DefaultSceneRoot`) (`self.Rotation`) false false)
        (`KismetSystemLibrary.Delay` 0.01)
        (goto _label_4))
      (else
        (set `self.PlayerMoved` true)
        (for _array_element (`self.Platforms`)
          (`/Engine/EditorBlueprintResources/StandardMacros.IsValid` _array_element
            (:`Is Valid`
              (`/Game/Blueprints/BP_Platform.PlayDetection` _array_element self (`KismetArrayLibrary.Array_Length` (`self.Platforms`)))
              (goto _label_3)))))))
  (:`Released`
    (set `self.RotatingRight` false)))

(event `Key|W`
  (params (Key :type "Key Structure"))
  (:`Pressed`
    (if (`self.PlayerMoved`)
      ;[0.07227 0 0.15 0.5] Rotate Up
      (set `self.RotatingUp` true :!label _label_5)
      (if (`self.RotatingUp`) :!label _label_6
        (set `self.Rotation` (struct :`Pitch` -1.0))
        (`SceneComponent.K2_AddWorldRotation` (`self.DefaultSceneRoot`) (`self.Rotation`) false false)
        (`KismetSystemLibrary.Delay` 0.01)
        (goto _label_6))
      (else
        (set `self.PlayerMoved` true)
        (for _array_element (`self.Platforms`)
          (`/Engine/EditorBlueprintResources/StandardMacros.IsValid` _array_element
            (:`Is Valid`
              (`/Game/Blueprints/BP_Platform.PlayDetection` _array_element self (`KismetArrayLibrary.Array_Length` (`self.Platforms`)))
              (goto _label_5)))))))
  (:`Released`
    (set `self.RotatingUp` false)))

(event `Key|S`
  (params (Key :type "Key Structure"))
  (:`Pressed`
    (if (`self.PlayerMoved`)
      ;[0.07617 0.15 0 0.5] Rotate Down
      (set `self.RotatingDown` true :!label _label_7)
      (if (`self.RotatingDown`) :!label _label_8
        (set `self.Rotation` (struct :`Pitch` 1.0))
        (`SceneComponent.K2_AddWorldRotation` (`self.DefaultSceneRoot`) (`self.Rotation`) false false)
        (`KismetSystemLibrary.Delay` 0.01)
        (goto _label_8))
      (else
        (set `self.PlayerMoved` true)
        (for _array_element (`self.Platforms`)
          (`/Engine/EditorBlueprintResources/StandardMacros.IsValid` _array_element
            (:`Is Valid`
              (`/Game/Blueprints/BP_Platform.PlayDetection` _array_element self (`KismetArrayLibrary.Array_Length` (`self.Platforms`)))
              (goto _label_7)))))))
  (:`Released`
    (set `self.RotatingDown` false)))

(event `PlayAnimation`
  ; Animation
  (`self.DisableInput` (`GameplayStatics.GetPlayerController` 0))
  (set `self.RotatingLeft` false)
  (set `self.RotatingRight` false)
  (set `self.RotatingUp` false)
  (set `self.RotatingDown` false)
  (`SceneComponent.K2_AddWorldOffset` (`self.ChildActor`) (/ (- (`SceneComponent.K2_GetComponentLocation` (`self.Door`)) (`SceneComponent.K2_GetComponentLocation` (`self.ChildActor`))) (50.0 50.0 50.0)) false false :!label _label_9)
  (`KismetSystemLibrary.Delay` 0.01)
  (if (== (`SceneComponent.K2_GetComponentLocation` (`self.Door`)) (`SceneComponent.K2_GetComponentLocation` (`self.ChildActor`)) :`ErrorTolerance` 0.5)
    (bind _returnvalue (`GameplayStatics.GetCurrentLevelName` true))
    (if (`KismetStringLibrary.EqualEqual_StrStr` _returnvalue "Level1")
      (`GameplayStatics.OpenLevelBySoftObjectPtr` "/Game/Level2.Level2")
      (else
        (`KismetSystemLibrary.QuitGame` null "Quit")))
    (else
      (goto _label_9))))

(fn `UserConstructionScript`
  (bind _outactors (`GameplayStatics.GetAllActorsOfClass` "/Game/Blueprints/BP_Platform.BP_Platform_C"))
  (set `self.Platforms` _outactors))