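; BP_Potions is a clickable potion prop that the player uses to distract the Witch.
; A click plays one of three random crystal sounds and calls Distraction with a Waypoint on the Witch's AIC_PathFollower AI controller.
; After a successful distraction, clicks are locked for a short cooldown.
; Hovering while clickable swaps all three potion meshes to a highlight material, and cursor exit restores the materials cached at BeginPlay.
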(event `self.ReceiveBeginPlay`
  (set `self.Potion1Mat` (`PrimitiveComponent.GetMaterial` (`self.Potion1`) 0))
  (set `self.Potion2Mat` (`PrimitiveComponent.GetMaterial` (`self.Potion2`) 0))
  (set `self.Potion3Mat` (`PrimitiveComponent.GetMaterial` (`self.Potion3`) 0)))

(event `self.ReceiveActorOnClicked`
  (params (ButtonPressed :type "Key Structure"))
  (if (`self.CanBeClicked`)
    ; Play Sounds
    (switch `int` (`KismetMathLibrary.RandomInteger` 3)
      (:`0`
        (`GameplayStatics.PlaySoundAtLocation` "/Game/Sound/Objects/Crystal_1.Crystal_1" (`self.K2_GetActorLocation`) (struct) 1.0 1.0 0.0 null null null null))
      (:`1`
        (`GameplayStatics.PlaySoundAtLocation` "/Game/Sound/Objects/Crystal_2.Crystal_2" (`self.K2_GetActorLocation`) (struct) 1.0 1.0 0.0 null null null null))
      (:`2`
        (`GameplayStatics.PlaySoundAtLocation` "/Game/Sound/Objects/Crystal_3.Crystal_3" (`self.K2_GetActorLocation`) (struct) 1.0 1.0 0.0 null null null null)))
    (bind _asaic_path_follower (cast `/Game/Blueprints/AI/AIC_PathFollower` (`AIBlueprintHelperLibrary.GetAIController` (`self.Witch`))))
    (`/Game/Blueprints/AI/AIC_PathFollower.Distraction` _asaic_path_follower (`self.Waypoint`))
    (set `self.CanBeClicked` false)
    (`KismetSystemLibrary.Delay` 5.0)
    (set `self.CanBeClicked` true)))

(event `self.ReceiveActorBeginCursorOver`
  (if (`self.CanBeClicked`)
    (`PrimitiveComponent.SetMaterial` (`self.Potion1`) 0 "/Game/Materials/Princess/M_coroa.M_coroa")
    (`PrimitiveComponent.SetMaterial` (`self.Potion2`) 0 "/Game/Materials/Princess/M_coroa.M_coroa")
    (`PrimitiveComponent.SetMaterial` (`self.Potion3`) 0 "/Game/Materials/Princess/M_coroa.M_coroa")))

(event `self.ReceiveActorEndCursorOver`
  (`PrimitiveComponent.SetMaterial` (`self.Potion1`) 0 (`self.Potion1Mat`))
  (`PrimitiveComponent.SetMaterial` (`self.Potion2`) 0 (`self.Potion2Mat`))
  (`PrimitiveComponent.SetMaterial` (`self.Potion3`) 0 (`self.Potion3Mat`)))

(fn `UserConstructionScript`)