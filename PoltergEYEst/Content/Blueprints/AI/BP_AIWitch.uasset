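; BP_AIWitch is an AI witch with a broom that turns toward a Sphere target and can become alerted on a game-over check.
; After a startup delay it takes a first yaw step, then a further delay sets IsLooking, letting Tick continue the interpolated turn each frame.
; While looking, CheckGameOver sets Alerted on the witch and broom Animation Blueprints.
; A call to start AIC_PathFollower walking is left disconnected.
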(event `self.ReceiveBeginPlay`
  (bind (_returnvalue_roll _returnvalue_pitch _returnvalue_yaw) (`KismetMathLibrary.BreakRotator` (`KismetMathLibrary.RInterpTo` (`self.K2_GetActorRotation`) (`KismetMathLibrary.FindLookAtRotation` (`self.K2_GetActorLocation`) (`self.K2_GetActorLocation` (`self.Sphere`))) (`GameplayStatics.GetWorldDeltaSeconds`) 2.0)))
  (`KismetSystemLibrary.Delay` 2.0)
  (`self.K2_SetActorRotation` (`KismetMathLibrary.MakeRotator` 0.0 0.0 _returnvalue_yaw) :!label _label)
  (`KismetSystemLibrary.Delay` 2.0)
  (set `self.IsLooking` true))

(event `self.ReceiveTick`
  (params (DeltaSeconds :type "Float (single-precision)"))
  (if (`self.IsLooking`)
    (goto _label)))

(event `CheckGameOver`
  ; Check GameOver
  (if (`self.IsLooking`)
    (bind _asab_witch (cast `/Game/Animations/Witch/AB_Witch` (`SkeletalMeshComponent.GetAnimInstance` (`self.Mesh`))))
    (set `/Game/Animations/Witch/AB_Witch.Alerted` true _asab_witch)
    (bind _asab_broom (cast `/Game/Animations/Broom/AB_Broom` (`SkeletalMeshComponent.GetAnimInstance` (`self.SkeletalMesh`))))
    (set `/Game/Animations/Broom/AB_Broom.Alerted` true _asab_broom)))

(fn `UserConstructionScript`)