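; AI controller that moves the witch along linked waypoints and triggers game over when she reaches the sphere waypoint.
; Each Tick compares move status to a desired status; on a mismatch it advances the target to NextWaypoint, or calls GameOver on the player character at the sphere.
; StartWalking issues a move to the current target, while StartRun retargets the witch straight to the sphere waypoint and moves there.
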(event `self.ReceiveBeginPlay`
  (bind _asbp_aiwitch (cast `/Game/Blueprints/AI/BP_AIWitch` (`self.K2_GetPawn`)))
  (set `self.StoredPawn` _asbp_aiwitch))

(event `self.ReceiveTick`
  (params (DeltaSeconds :type "Float (single-precision)"))
  (bind _storedpawn (`self.StoredPawn`))
  (bind _storedpawn_2 (`self.StoredPawn`))
  ; IsStopped?
  (if (`|EnumInequality` (`self.GetMoveStatus`) (`self.DesiredStatus`))
    (if (== (`/Game/Blueprints/AI/BP_AIWitch.TargetWaypoint` _storedpawn_2) (`/Game/Blueprints/AI/BP_AIWitch.SphereWaypoint` _storedpawn_2))
      (bind _asbp_first_person_character (cast `/Game/FirstPerson/Blueprints/BP_FirstPersonCharacter` (`GameplayStatics.GetPlayerPawn` 0)))
      (`/Game/FirstPerson/Blueprints/BP_FirstPersonCharacter.GameOver` _asbp_first_person_character)
      (else
        (bind _output_get (set `/Game/Blueprints/AI/BP_AIWitch.TargetWaypoint` (`/Game/Blueprints/AIHelpers/BP_Waypoint.NextWaypoint` (`/Game/Blueprints/AI/BP_AIWitch.TargetWaypoint` _storedpawn)) _storedpawn))))))

(event `StartWalking`
  ; Start Walking
  (`self.MoveToActor` (stale `self.ReceiveTick` _output_get) 15.0 true true true null))

(event `StartRun`
  (bind _storedpawn (`self.StoredPawn`))
  (bind _output_get (set `/Game/Blueprints/AI/BP_AIWitch.TargetWaypoint` (`/Game/Blueprints/AI/BP_AIWitch.SphereWaypoint` _storedpawn) _storedpawn))
  (`self.MoveToActor` _output_get 15.0 true true true null))

(fn `UserConstructionScript`)