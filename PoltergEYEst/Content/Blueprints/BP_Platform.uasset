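; Platform actor that tests, with debug traces, what lies between its four top vertices and the camera.
; From BeginPlay it loops every two seconds; while PlayerMoved is true, it line-traces from each vertex to CameraActor and prints the hit component's name.
; The construction script caches a level CameraActor and fills ActorsToIgnore with spheres and rifle pickups, though the traces do not use that list.
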(event `self.ReceiveBeginPlay`
  (if (`self.PlayerMoved`) :!label _label
    (bind _outhit (`KismetSystemLibrary.LineTraceSingle` :`Start` (`SceneComponent.K2_GetComponentLocation` (`self.TopVertice1`)) :`End` (`self.K2_GetActorLocation` (`self.CameraActor`)) :`TraceChannel` "TraceTypeQuery3" :`DrawDebugType` "ForDuration" :`DrawTime` 2.0))
    (`KismetSystemLibrary.PrintString` (`KismetSystemLibrary.GetDisplayName` (`.HitComponent` (`GameplayStatics.BreakHitResult` _outhit))))
    (bind _outhit_2 (`KismetSystemLibrary.LineTraceSingle` :`Start` (`SceneComponent.K2_GetComponentLocation` (`self.TopVertice2`)) :`End` (`self.K2_GetActorLocation` (`self.CameraActor`)) :`TraceChannel` "TraceTypeQuery3" :`DrawDebugType` "ForDuration" :`DrawTime` 2.0))
    (`KismetSystemLibrary.PrintString` (`KismetSystemLibrary.GetDisplayName` (`.HitComponent` (`GameplayStatics.BreakHitResult` _outhit_2))))
    (bind _outhit_3 (`KismetSystemLibrary.LineTraceSingle` :`Start` (`SceneComponent.K2_GetComponentLocation` (`self.TopVertice3`)) :`End` (`self.K2_GetActorLocation` (`self.CameraActor`)) :`TraceChannel` "TraceTypeQuery3" :`DrawDebugType` "ForDuration" :`DrawTime` 2.0))
    (`KismetSystemLibrary.PrintString` (`KismetSystemLibrary.GetDisplayName` (`.HitComponent` (`GameplayStatics.BreakHitResult` _outhit_3))))
    (bind _outhit_4 (`KismetSystemLibrary.LineTraceSingle` :`Start` (`SceneComponent.K2_GetComponentLocation` (`self.TopVertice4`)) :`End` (`self.K2_GetActorLocation` (`self.CameraActor`)) :`TraceChannel` "TraceTypeQuery3" :`DrawDebugType` "ForDuration" :`DrawTime` 2.0))
    (`KismetSystemLibrary.PrintString` (`KismetSystemLibrary.GetDisplayName` (`.HitComponent` (`GameplayStatics.BreakHitResult` _outhit_4)))))
  (`KismetSystemLibrary.Delay` 2.0)
  (goto _label))

(fn `UserConstructionScript`
  (bind _actors_to_ignore (`self.Actors to Ignore`))
  (bind _outactors (`GameplayStatics.GetAllActorsOfClass` "/Script/Engine.CameraActor"))
  (for _array_element _outactors
    _)
  (`/Engine/EditorBlueprintResources/StandardMacros.IsValid` _array_element
    (:`Is Valid`
      (set `self.CameraActor` _array_element)
      (bind _outactors_2 (`GameplayStatics.GetAllActorsOfClass` "/Game/Blueprints/BP_Sphere.BP_Sphere_C"))
      (for _array_element_2 _outactors_2
        (`/Engine/EditorBlueprintResources/StandardMacros.IsValid` _array_element_2
          (:`Is Valid`
            (`KismetArrayLibrary.Array_Add` _actors_to_ignore _array_element_2)
            (bind _outactors_3 (`GameplayStatics.GetAllActorsOfClass` "/Game/FirstPerson/Blueprints/BP_PickUp_Rifle.BP_PickUp_Rifle_C"))
            (for _array_element_3 _outactors_3
              (`/Engine/EditorBlueprintResources/StandardMacros.IsValid` _array_element_3
                (:`Is Valid`
                  (`KismetArrayLibrary.Array_Add` _actors_to_ignore _array_element_3))))))))))